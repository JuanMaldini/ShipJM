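; Bp_Gun is a projectile actor that scales itself through a Grow timeline on spawn and launches toward a target point.
; ImpulsetoEnemy2 enables physics on its Sphere and applies a unit-direction impulse toward GoTo, with no force multiplier.
; A Sphere hit triggers a light-blast Niagara effect and destroys the actor.
; Otherwise, a delay after launch spawns Bp_Explosion at the actor's location, then destroys it.
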(event `self.ReceiveBeginPlay`
  (bind (_direction _grow) (`Timeline|Grow`)
    (:`Update`
      (`self.SetActorRelativeScale3D` (`KismetMathLibrary.Conv_DoubleToVector` _grow)))))

(event `self.Sphere.OnComponentHit`
  (params (HitComponent :type "PrimitiveComponent Object Reference") (OtherActor :type "Actor Object Reference") (OtherComp :type "PrimitiveComponent Object Reference") (NormalImpulse :type "Vector Structure") (Hit :type "HitResult Structure (by ref)"))
  (`NiagaraFunctionLibrary.SpawnSystemAttached` "/Game/MegaMagicVFXBundle/VFX/MagicalExplosionsVFX/VFX/LightBlast/Systems/N_LightBlast1.N_LightBlast1" null "None" (`SceneComponent.K2_GetComponentLocation` (`self.Sphere`)) (struct) "KeepRelativeOffset")
  (`self.K2_DestroyActor`))

(event `Impulse to Enemy2`
  (params (`Go To` :type "Vector Structure"))
  (bind _sphere (`self.Sphere`))
  (`PrimitiveComponent.SetSimulatePhysics` _sphere true)
  (`PrimitiveComponent.AddImpulse` _sphere (`KismetMathLibrary.GetDirectionUnitVector` (`SceneComponent.K2_GetComponentLocation` _sphere) `Go To`) "None" false)
  (`KismetSystemLibrary.Delay` 3.0)
  (`|SpawnActorFromClass` "/Game/Blueprint/Bp_Explosion.Bp_Explosion_C" (`KismetMathLibrary.MakeTransform` (`self.K2_GetActorLocation`)) "Undefined" "MultiplyWithRoot" null null)
  (`self.K2_DestroyActor`))

(fn `UserConstructionScript`)