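; Player ship pawn that climbs automatically to a height cap and fights Bp_Enemy actors.
; The MoveUp axis adjusts the climb and Niagara exhaust, with negative input halting upward thrust.
; A timeline charges the gun; Fire launches the Bp_Gun fireball at a random enemy, then spawns a replacement after a delay.
; Random damage depletes life until the ship explodes and notifies its controller; F and R keys trigger test damage.
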(event `self.ReceiveBeginPlay`
  (`|ExecutionSequence`
    (:`then_0`
      (bind _asbp_ship_controller (cast `/Game/Blueprint/Bp_Ship_Controller` (`self.GetController`)))
      (set `self.Bp Ship Controller` _asbp_ship_controller))
    (:`then_1`
      (set `self.CanFire` true))
    (:`then_2`
      (bind _returnvalue (`|SpawnActorFromClass` "/Game/Blueprint/Bp_Gun.Bp_Gun_C" (`KismetMathLibrary.MakeTransform` (0.0 -111.428571 3942.856941)) "Undefined" "MultiplyWithRoot" null null))
      (set `self.FireBall` _returnvalue))
    (:`then_3`
      (`self.ChargeGun`))))

(event `self.ReceiveTick`
  (params (DeltaSeconds :type "Float (single-precision)"))
  ;[0 0 0 0.5] Movement
  (set `self.MyHeigth` (.z (`self.K2_GetActorLocation`)))
  (if (`/Game/Blueprint/Bp_Ship_Controller.Finish?` (`self.Bp Ship Controller`))
    _
    (elif (`self.GoDown`)
      _
      (elif (not (`self.Get Max Heigth`))
        (`self.AddMovementInput` (0.0 0.0 1.0) 0.1)))))

(event `Key|F`
  (params (Key :type "Key Structure"))
  ;[0 0 0 0.5] Make Damage
  (:`Pressed`
    (`self.Damage_Receive`)))

(event `InputAxis|MoveUp`
  (params (AxisValue :type "Float (single-precision)"))
  ;[0 0 0 0.5] Movement
  (`self.NiagaraBoost` AxisValue)
  (if (<= AxisValue -0.5)
    (set `self.GoDown` true)
    (else
      (set `self.GoDown` false)))
  (if (`self.GoDown`)
    _
    (elif (not (`self.Get Max Heigth`))
      (`self.AddMovementInput` (0.0 0.0 1.0) (* AxisValue 0.5)))))

(event `Key|R`
  (params (Key :type "Key Structure"))
  ;[0 0 0 0.5] Make Damage to Enemy
  (:`Pressed`
    (bind _returnvalue (`GameplayStatics.GetActorOfClass` "/Game/Blueprint/Enemy/Bp_Enemy.Bp_Enemy_C"))
    (`/Game/Blueprint/Enemy/Bp_Enemy.Damage_Receive` _returnvalue)))

(event `ChargeGun`
  (bind (_direction _charge) (`Timeline|Gun` :!via `PlayFromStart`)
    (:`Update`
      (set `self.ValueCharge` _charge))
    (:`Finished`
      (set `self.IsChargedGun` true))))

(event `InputAction|Fire`
  (params (Key :type "Key Structure"))
  (:`Pressed`
    (if (`self.CanFire`)
      (if (`self.IsChargedGun`)
        (set `self.IsChargedGun` false)
        (set `self.ValueCharge` 0.0)
        (bind _go_to (`self.FindEnemy`))
        (`self.FireNiagara` _go_to)
        (`KismetSystemLibrary.PrintString` "FIRE")
        (`self.ChargeGun`)
        (`KismetSystemLibrary.Delay` 3.0)
        (bind _returnvalue (`|SpawnActorFromClass` "/Game/Blueprint/Bp_Gun.Bp_Gun_C" (`KismetMathLibrary.MakeTransform` (0.0 -111.428571 3942.856941)) "Undefined" "MultiplyWithRoot" null null))
        (bind _output_get (set `self.FireBall` _returnvalue))
        (`self.K2_AttachToComponent` _output_get (`self.CollisionComponent`) "None" "KeepRelative" "KeepRelative" "KeepRelative" true)
        (else
          (`KismetSystemLibrary.PrintString` "Charging..."))))))

(event `self.SphereCollision.OnComponentHit`
  (params (HitComponent :type "PrimitiveComponent Object Reference") (OtherActor :type "Actor Object Reference") (OtherComp :type "PrimitiveComponent Object Reference") (NormalImpulse :type "Vector Structure") (Hit :type "HitResult Structure (by ref)"))
  (if (== OtherActor "/Game/Blueprint/Enemy/Bp_Enemy.Bp_Enemy")
    (`self.K2_DestroyActor`)))

(fn `Damage_Receive`
  (if (not (<= (`self.Life_Ship`) 0.0))
    (set `self.Life_Ship` (- (`self.Life_Ship`) (`KismetMathLibrary.RandomFloatInRange` 0.15 0.3)))
    (if (not (<= (`self.Life_Ship`) 0.0))
      (return)
      (else
        _)))
  (`/Game/Blueprint/Bp_Ship_Controller.Finish` (`self.Bp Ship Controller`))
  (set `self.CanFire` false)
  (`self.Explosion`)
  (`self.K2_DestroyActor`))

(fn `Explosion`
  (bind _returnvalue (`self.K2_GetActorLocation`))
  (`SceneComponent.K2_SetRelativeTransform` (`self.MeshComponent`) (`KismetMathLibrary.MakeTransform` _returnvalue) false false)
  (`|SpawnActorFromClass` "/Game/Blueprint/Bp_Explosion.Bp_Explosion_C" (`KismetMathLibrary.MakeTransform` _returnvalue) "Undefined" "MultiplyWithRoot" null null))

(fn `FindEnemy`
  (returns (`Go to` :type "Vector Structure"))
  (bind _outactors (`GameplayStatics.GetAllActorsOfClass` "/Game/Blueprint/Enemy/Bp_Enemy.Bp_Enemy_C"))
  (return (`self.K2_GetActorLocation` (`KismetArrayLibrary.Array_Random` _outactors))))

(fn `FireNiagara`
  (params (`Enemy location` :type "Vector Structure"))
  (`/Game/Blueprint/Bp_Gun.Impulse to Enemy` (`self.FireBall`) `Enemy location`)
  (return))

(fn `Get Max Heigth`
  (returns (`Is Max Heigth` :type Boolean))
  (bind (_returnvalue_x _returnvalue_y _returnvalue_z) (`KismetMathLibrary.BreakVector` (`self.K2_GetActorLocation`)))
  (return (>= _returnvalue_z 10000.0)))

(fn `NiagaraBoost`
  (params (input :type "Float (double-precision)"))
  (bind _ns_rocketexhaust_realistic1 (`self.NS_RocketExhaust_Realistic1`))
  (if (>= input 0.5)
    (`NiagaraComponent.SetVariableFloat` _ns_rocketexhaust_realistic1 "Thrusters_Speed" 3000.0)
    (`NiagaraComponent.SetVariableFloat` _ns_rocketexhaust_realistic1 "Emissive_Boost" 10.0)
    (`NiagaraComponent.SetVariableFloat` _ns_rocketexhaust_realistic1 "Particulate_Speed" 1000.0)
    (else
      (`NiagaraComponent.SetVariableFloat` _ns_rocketexhaust_realistic1 "Thrusters_Speed" 800.0)
      (`NiagaraComponent.SetVariableFloat` _ns_rocketexhaust_realistic1 "Emissive_Boost" 1.0)
      (`NiagaraComponent.SetVariableFloat` _ns_rocketexhaust_realistic1 "Particulate_Speed" 400.0)))
  (return))

(fn `UserConstructionScript`)