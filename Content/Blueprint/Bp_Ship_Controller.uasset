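; Player controller for the ship game that creates the HUD, tracks the match result and keeps win/loss totals.
; Tick ends the match once the ship pawn reaches a height threshold, guarded by a one-shot flag.
; Finish counts a win at that height or a loss otherwise, shows the end-match widget and saves.
; Totals load on BeginPlay and save through the game instance, with a separate event to reset them.
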(event `self.ReceiveBeginPlay`
  (`|ExecutionSequence`
    (:`then_0`
      (bind _asbp_ship_pawn (cast `/Game/Blueprint/Bp_Ship_Pawn` (`self.K2_GetPawn`)))
      (set `self.As Bp Ship Pawn` _asbp_ship_pawn))
    (:`then_1`
      (bind _returnvalue (`|CreateWidget` "/Game/Blueprint/W_Ship.W_Ship_C"))
      (bind _output_get (set `self.W_Ship` _returnvalue))
      (`UserWidget.AddToViewport` _output_get 0))
    (:`then_2`
      (set `self.bShowMouseCursor` true))
    (:`then_3`
      (`KismetSystemLibrary.ExecuteConsoleCommand` "r.Streaming.PoolSize 12000" null))
    (:`then_4`
      (set `/Game/Blueprint/W_Ship.WatchHeigth` true (`self.W_Ship`))
      (set `self.oneTime` true))
    (:`then_5`
      (`self.LoadData`))))

(event `LoadData`
  ;[0 0 0 0.5] Load Data
  (bind _asbp_game_instance (cast `/Game/Blueprint/Save/Bp_GameInstance` (`GameplayStatics.GetGameInstance`)))
  (bind _asbp_save_game (`/Game/Blueprint/Save/Bp_GameInstance.LoadGame` _asbp_game_instance "MyFileName"))
  (`/Engine/EditorBlueprintResources/StandardMacros.IsValid` _asbp_save_game
    (:`Is Valid`
      (`|ExecutionSequence`
        (:`then_0`
          (set `self.Win_Games` (`/Game/Blueprint/Save/Bp_SaveGame.Win` _asbp_save_game)))
        (:`then_1`
          (set `self.Loose_Games` (`/Game/Blueprint/Save/Bp_SaveGame.Loose` _asbp_save_game)))))))

(event `SaveData`
  ;[0 0 0 0.5] SaveData
  (bind _asbp_game_instance (cast `/Game/Blueprint/Save/Bp_GameInstance` (`GameplayStatics.GetGameInstance`)))
  (bind _returnvalue (`GameplayStatics.CreateSaveGameObject` "/Game/Blueprint/Save/Bp_SaveGame.Bp_SaveGame_C"))
  (set `/Game/Blueprint/Save/Bp_SaveGame.Win` (`self.Win_Games`) _returnvalue)
  (set `/Game/Blueprint/Save/Bp_SaveGame.Loose` (`self.Loose_Games`) _returnvalue)
  (`/Game/Blueprint/Save/Bp_GameInstance.SaveGame` _asbp_game_instance _returnvalue "MyFileName" true))

(event `ResetData`
  ;[0 0 0 0.5] Reset Data
  (bind _asbp_game_instance (cast `/Game/Blueprint/Save/Bp_GameInstance` (`GameplayStatics.GetGameInstance`)))
  (bind _returnvalue (`GameplayStatics.CreateSaveGameObject` "/Game/Blueprint/Save/Bp_SaveGame.Bp_SaveGame_C"))
  (set `/Game/Blueprint/Save/Bp_SaveGame.Win` 0 _returnvalue)
  (set `/Game/Blueprint/Save/Bp_SaveGame.Loose` 0 _returnvalue)
  (`/Game/Blueprint/Save/Bp_GameInstance.SaveGame` _asbp_game_instance _returnvalue "MyFileName" true)
  (`KismetSystemLibrary.PrintString` "WIN: 0 / LOOSE: 0"))

(event `self.ReceiveTick`
  (params (DeltaSeconds :type "Float (single-precision)"))
  ;[0 0 0 0.5] Watch Heigth Ship
  (if (and (`self.is Max Heigth`) (`self.oneTime`))
    (set `self.oneTime` false)
    (`self.Finish`)))

(event `Finish`
  ;[0 0 0 0.5] When finish
  (`|ExecutionSequence`
    (:`then_0`
      (`self.UpdateWinOrLoose`)
      (set `self.Finish?` true))
    (:`then_1`
      (set `/Game/Blueprint/W_Ship.WatchHeigth` false (`self.W_Ship`)))
    (:`then_2`
      (bind _returnvalue (`|CreateWidget` "/Game/Blueprint/W_EndMatch.W_EndMatch_C"))
      (`UserWidget.AddToViewport` _returnvalue 0))
    (:`then_3`
      (`self.SaveData`))))

(fn `is Max Heigth`
  (returns (NewParam :type Boolean))
  (bind (_returnvalue_x _returnvalue_y _returnvalue_z) (`KismetMathLibrary.BreakVector` (`self.K2_GetActorLocation` (`self.As Bp Ship Pawn`))))
  (return (>= _returnvalue_z 10000.0)))

(fn `UpdateWinOrLoose`
  (if (`self.is Max Heigth`)
    (`/Engine/EditorBlueprintResources/StandardMacros.IncrementInt` (`self.Win_Games`))
    (else
      (`/Engine/EditorBlueprintResources/StandardMacros.IncrementInt` (`self.Loose_Games`)))))

(fn `UserConstructionScript`)