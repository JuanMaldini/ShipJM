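; Enemy actor that relocates on BeginPlay, takes random damage and respawns a replacement when killed.
; NewLocation stores a random Y/Z offset position, spawns a Bp_NewLocation actor and moves the collision component, re-rolling the randoms for each.
; DamageReceive lowers life; at zero it spawns an explosion, a new Bp_Enemy at the stored position, then destroys itself and that actor.
; Any overlap or hit destroys the enemy without respawning.
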(event `self.ReceiveBeginPlay`
  (`self.NewLocation`))

(event `self.CollisionComponent.OnComponentBeginOverlap`
  (params (OverlappedComponent :type "PrimitiveComponent Object Reference") (OtherActor :type "Actor Object Reference") (OtherComp :type "PrimitiveComponent Object Reference") (OtherBodyIndex :type Integer) (bFromSweep :type Boolean) (SweepResult :type "HitResult Structure (by ref)"))
  (`KismetSystemLibrary.PrintString` "ENEMY OVERLAP")
  (`self.K2_DestroyActor` :!label _label))

(event `self.CollisionComponent.OnComponentHit`
  (params (HitComponent :type "PrimitiveComponent Object Reference") (OtherActor :type "Actor Object Reference") (OtherComp :type "PrimitiveComponent Object Reference") (NormalImpulse :type "Vector Structure") (Hit :type "HitResult Structure (by ref)"))
  (`KismetSystemLibrary.PrintString` "ENEMY HIT")
  (goto _label))

(fn `Damage_Receive`
  (if (not (<= (`self.Life_Enemy`) 0.0))
    (set `self.Life_Enemy` (- (`self.Life_Enemy`) (`KismetMathLibrary.RandomFloatInRange` 0.15 0.3)))
    (if (not (<= (`self.Life_Enemy`) 0.0))
      (return)
      (else
        _)))
  (`self.Explosion`)
  (`|SpawnActorFromClass` "Bp_Enemy_C" (`KismetMathLibrary.MakeTransform` (`self.NewLocationEnemy`)) "Undefined" "MultiplyWithRoot" null null)
  (`self.K2_DestroyActor`)
  (`self.K2_DestroyActor` (`self.NewLocationRef`)))

(fn `Explosion`
  (bind _returnvalue (`self.K2_GetActorLocation`))
  (`SceneComponent.K2_SetRelativeTransform` (`self.MeshComponent`) (`KismetMathLibrary.MakeTransform` _returnvalue) false false)
  (`|SpawnActorFromClass` "/Game/Blueprint/Bp_Explosion.Bp_Explosion_C" (`KismetMathLibrary.MakeTransform` _returnvalue) "Undefined" "MultiplyWithRoot" null null)
  (return))

(fn `NewLocation`
  (bind (_returnvalue_x _returnvalue_y _returnvalue_z) (`KismetMathLibrary.BreakVector` (`SceneComponent.K2_GetComponentLocation` (`self.CollisionComponent`))))
  (bind _returnvalue (`KismetMathLibrary.MakeVector` _returnvalue_x (- _returnvalue_y (`KismetMathLibrary.RandomFloatInRange` -4000.0 4000.0)) (- _returnvalue_z (`KismetMathLibrary.RandomFloatInRange` -4000.0 4000.0))))
  (set `self.NewLocationEnemy` _returnvalue)
  (bind _returnvalue_2 (`|SpawnActorFromClass` "/Game/Blueprint/Enemy/Bp_NewLocation.Bp_NewLocation_C" (`KismetMathLibrary.MakeTransform` _returnvalue (struct) (3.0 3.0 3.0)) "Undefined" "MultiplyWithRoot" null null))
  (set `self.NewLocationRef` _returnvalue_2)
  (`SceneComponent.K2_SetWorldLocation` (`self.CollisionComponent`) _returnvalue false false)
  (return))

(fn `Update Life Enemy`)

(fn `UserConstructionScript`)